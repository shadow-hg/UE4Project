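; Test actor that stretches two plane meshes between a BeginPoint and an EndPoint actor, forming a beam-like connection.
; Both planes sit at the midpoint, scale in X by the distance between the points, and face along the connecting line.
; Plane gets an extra 90-degree roll, so the pair forms a cross visible from multiple angles.
; The same logic runs in the construction script for editor preview and every Tick to follow moving endpoints.
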(event EventBeginPlay)

(event Collision|EventActorBeginOverlap
  (params (OtherActor :type Actor%20Object%20Reference)))

(event EventTick
  (params (DeltaSeconds :type Float%20%28single-precision%29))
  (bind _plane1 (Variables|Default|GetPlane1))
  (bind _endpoint (Variables|Default|GetEndPoint))
  (bind _beginpoint (Variables|Default|GetBeginPoint))
  (bind _endpoint_2 (Variables|Default|GetEndPoint))
  (bind _beginpoint_2 (Variables|Default|GetBeginPoint))
  (bind _plane (Variables|Default|GetPlane))
  (bind _returnvalue (Transformation|GetActorLocation _endpoint_2))
  (bind _returnvalue_2 (Transformation|GetActorLocation _beginpoint_2))
  (bind _returnvalue_3 (Transformation|GetActorLocation _beginpoint))
  (bind _returnvalue_4 (Transformation|GetActorLocation _endpoint))
  (bind _returnvalue_5 (Math|Rotator|FindLookatRotation _returnvalue _returnvalue_2))
  (bind _returnvalue_6 (Math|Rotator|FindLookatRotation _returnvalue_4 _returnvalue_3))
  (Utilities|FlowControl|Sequence
    (:then_0
      (Transformation|SetWorldLocation _plane (* (+ _returnvalue _returnvalue_2) 0.5) false false)
      (Transformation|SetWorldScale3D _plane (Math|Vector|MakeVector (/ (Math|Vector|Distance(Vector) _returnvalue _returnvalue_2) 1e+02) 1.0 1.0))
      (Transformation|SetWorldRotation _plane (Math|Rotator|MakeRotator (+ (.roll _returnvalue_5) 9e+01) (.pitch _returnvalue_5) (.yaw _returnvalue_5)) false false))
    (:then_1
      (Transformation|SetWorldLocation _plane1 (* (+ _returnvalue_4 _returnvalue_3) 0.5) false false)
      (Transformation|SetWorldScale3D _plane1 (Math|Vector|MakeVector (/ (Math|Vector|Distance(Vector) _returnvalue_4 _returnvalue_3) 1e+02) 1.0 1.0))
      (Transformation|SetWorldRotation _plane1 (Math|Rotator|MakeRotator (.roll _returnvalue_6) (.pitch _returnvalue_6) (.yaw _returnvalue_6)) false false))))

(fn ConstructionScript
  (bind _plane1 (Variables|Default|GetPlane1))
  (bind _endpoint (Variables|Default|GetEndPoint))
  (bind _beginpoint (Variables|Default|GetBeginPoint))
  (bind _endpoint_2 (Variables|Default|GetEndPoint))
  (bind _beginpoint_2 (Variables|Default|GetBeginPoint))
  (bind _plane (Variables|Default|GetPlane))
  (bind _returnvalue (Transformation|GetActorLocation _endpoint_2))
  (bind _returnvalue_2 (Transformation|GetActorLocation _beginpoint_2))
  (bind _returnvalue_3 (Transformation|GetActorLocation _beginpoint))
  (bind _returnvalue_4 (Transformation|GetActorLocation _endpoint))
  (bind _returnvalue_5 (Math|Rotator|FindLookatRotation _returnvalue _returnvalue_2))
  (bind _returnvalue_6 (Math|Rotator|FindLookatRotation _returnvalue_4 _returnvalue_3))
  (Utilities|FlowControl|Sequence
    (:then_0
      (Transformation|SetWorldLocation _plane (* (+ _returnvalue _returnvalue_2) 0.5) false false)
      (Transformation|SetWorldScale3D _plane (Math|Vector|MakeVector (/ (Math|Vector|Distance(Vector) _returnvalue _returnvalue_2) 1e+02) 1.0 1.0))
      (Transformation|SetWorldRotation _plane (Math|Rotator|MakeRotator (+ (.roll _returnvalue_5) 9e+01) (.pitch _returnvalue_5) (.yaw _returnvalue_5)) false false))
    (:then_1
      (Transformation|SetWorldLocation _plane1 (* (+ _returnvalue_4 _returnvalue_3) 0.5) false false)
      (Transformation|SetWorldScale3D _plane1 (Math|Vector|MakeVector (/ (Math|Vector|Distance(Vector) _returnvalue_4 _returnvalue_3) 1e+02) 1.0 1.0))
      (Transformation|SetWorldRotation _plane1 (Math|Rotator|MakeRotator (.roll _returnvalue_6) (.pitch _returnvalue_6) (.yaw _returnvalue_6)) false false))))